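; BP_Door is an interactable door that toggles DoorPivot between closed and OpenAngle rotations instantly when Interact fires.
; Opening and closing are gated by either the player character's TerminalUnlocked flag, when RequiresTerminalUnlock is set, or otherwise by IsLocked, with debug messages reporting the result.
; GetInteractionText picks locked, open or close prompts, but its terminal-lock branch is disconnected and never runs.
; CanInteract always returns true.
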(event EventBeginPlay)

(event Collision|EventActorBeginOverlap
  (params (OtherActor :type Actor%20Object%20Reference)))

(event EventTick
  (params (DeltaSeconds :type Float%20%28single-precision%29)))

(event EventInteract
  (if (Variables|Default|GetbRequiresTerminalUnlock)
    (bind _asbp_first_person_character (Utilities|Casting|CastToBP_FirstPersonCharacter (Game|GetPlayerCharacter 0)))
    (if (Variables|/Game/FirstPerson/Blueprints/BP_FirstPersonCharacter.BP_FirstPersonCharacter_C|GetTerminalUnlocked _asbp_first_person_character)
      (if (Variables|Door|GetbIsOpen) :!label _label
        (Transformation|SetRelativeRotation (Variables|Default|GetDoorPivot) "0, 0, 0" false false)
        (Variables|Door|SetbIsOpen false)
        (Development|PrintString "Door is closed")
        (else
          (Transformation|SetRelativeRotation (Variables|Default|GetDoorPivot) (Variables|Door|GetOpenAngle) false false)
          (Variables|Door|SetbIsOpen true)
          (Development|PrintString "Door is opened")))
      (else
        (Development|PrintString "Requires terminal access")))
    (elif (Variables|Door|GetbIsLocked)
      (Development|PrintString "Door is locked")
      (else
        (goto _label)))))

(fn ConstructionScript)

(fn CanInteract
  (return true))

(fn GetInteractionText
  (if (Variables|Door|GetbIsLocked)
    (return (Variables|Door|GetLockedPromptText))
    (elif (Variables|Door|GetbIsOpen)
      (return (Variables|Door|GetClosePromptText))
      (else
        (return (Variables|Door|GetOpenPromptText))))))