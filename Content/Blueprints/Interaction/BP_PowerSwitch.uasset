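; BP_PowerSwitch is an interactable switch that restores power when the player has a fuse.
; On Interact it casts the player character to BP_FirstPersonCharacter and, if HasFuse is set, sets PowerRestored on that character.
; Otherwise it reports that a fuse is needed, with both outcomes shown only through debug prints.
; CanInteract always returns true, and GetInteractionText supplies the "Restore power [E]" prompt.
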(event EventBeginPlay)

(event Collision|EventActorBeginOverlap
  (params (OtherActor :type Actor%20Object%20Reference)))

(event EventTick
  (params (DeltaSeconds :type Float%20%28single-precision%29)))

(event EventInteract
  ;[1 1 1] Comment
  (bind _asbp_first_person_character (Utilities|Casting|CastToBP_FirstPersonCharacter (Game|GetPlayerCharacter 0)))
  (if (Variables|/Game/FirstPerson/Blueprints/BP_FirstPersonCharacter.BP_FirstPersonCharacter_C|GetHasFuse _asbp_first_person_character)
    (Variables|/Game/FirstPerson/Blueprints/BP_FirstPersonCharacter.BP_FirstPersonCharacter_C|SetPowerRestored _asbp_first_person_character true)
    (Development|PrintString "Power restored")
    (else
      (Development|PrintString "Need fuse"))))

(fn ConstructionScript)

(fn CanInteract
  (return true))

(fn GetInteractionText
  (return "Restore power [E]"))