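; BP_Terminal is an interactable terminal that the player uses to set a terminal-unlocked state, provided power has been restored.
; Interact casts the player to BP_FirstPersonCharacter and checks its PowerRestored flag, then either sets TerminalUnlocked on that character or reports no power via a debug print.
; CanInteract always allows use and GetInteractionText supplies the prompt, so progression state lives on the character rather than the terminal.
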(event EventBeginPlay)

(event Collision|EventActorBeginOverlap
  (params (OtherActor :type Actor%20Object%20Reference)))

(event EventTick
  (params (DeltaSeconds :type Float%20%28single-precision%29)))

(event EventInteract
  (bind _asbp_first_person_character (Utilities|Casting|CastToBP_FirstPersonCharacter (Game|GetPlayerCharacter 0)))
  (if (Variables|/Game/FirstPerson/Blueprints/BP_FirstPersonCharacter.BP_FirstPersonCharacter_C|GetPowerRestored _asbp_first_person_character)
    (Variables|/Game/FirstPerson/Blueprints/BP_FirstPersonCharacter.BP_FirstPersonCharacter_C|SetTerminalUnlocked _asbp_first_person_character true)
    (Development|PrintString "Terminal unlocked")
    (else
      (Development|PrintString "No power"))))

(fn ConstructionScript)

(fn CanInteract
  (return true))

(fn GetInteractionText
  (return "Use terminal [E]"))